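; BP_Bullet is a six-second projectile that moves along world negative X each tick, faster when IsHitted is true, and enables overlaps after a short delay.
; Touching a firing FirstPersonCharacter turns it into a physics body, kicked by a forward impulse plus the player's sideways velocity, with a one-time sound.
; Touching a non-firing player calls Death, while touching a BP_Enemy calls Interaction; both destroy the bullet.
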(event OnComponentBeginOverlap(SphereCollision)
  (params (OverlappedComponent :type Primitive%20Component%20Object%20Reference) (OtherActor :type Actor%20Object%20Reference) (OtherComp :type Primitive%20Component%20Object%20Reference) (OtherBodyIndex :type Integer) (bFromSweep :type Boolean) (SweepResult :type Hit%20Result%20Structure%20%28by%20ref%29))
  (bind _asfirst_person_character (Utilities|Casting|CastToFirstPersonCharacter OtherActor)
    (:then
      (if (Variables|/Game/FirstPersonBP/Blueprints/FirstPersonCharacter.FirstPersonCharacter_C|GetIsFiring _asfirst_person_character)
        (Physics|SetSimulatePhysics (Variables|Default|GetSphere) true)
        (Collision|SetCollisionEnabled (Variables|Default|GetSphereCollision) "QueryAndPhysics")
        (Transformation|AttachComponentToComponent (Variables|Default|GetSphere) (Variables|Default|GetSphereCollision) "None" "KeepWorld" "KeepWorld" "KeepWorld" true)
        (Physics|AddImpulse (Variables|Default|GetSphere) (Math|Vector|MakeVector (.x (* (Transformation|GetActorForwardVector) 5e+03)) (* (.y (Variables|/Script/Engine.MovementComponent|GetVelocity (Variables|/Script/Engine.Character|GetCharacterMovement _asfirst_person_character))) 5.0) 0.0) "None" false)
        (Utilities|FlowControl|DoOnce false
          (:Completed
            (Audio|PlaySound2D "/Game/Sounds/C_Kick.C_Kick" 1.0 1.0 0.0 0 0)))
        (else
          (Default|Death _asfirst_person_character)
          (Actor|DestroyActor))))
    (:CastFailed
      (bind _asbp_enemy (Utilities|Casting|CastToBP_Enemy OtherActor))
      (Default|Interaction _asbp_enemy)
      (Actor|DestroyActor))))

(event EventBeginPlay
  (Actor|SetLifeSpan 6.0)
  (Variables|/Script/Engine.PrimitiveComponent|SetbGenerateOverlapEvents (Variables|Default|GetSphereCollision) false)
  (Utilities|FlowControl|Delay 0.5)
  (Variables|/Script/Engine.PrimitiveComponent|SetbGenerateOverlapEvents (Variables|Default|GetSphereCollision) true))

(event EventTick
  (params (DeltaSeconds :type Float%20%28single-precision%29))
  (Transformation|AddActorWorldOffset (Math|Vector|MakeVector (+ (* DeltaSeconds (Math|Float|SelectFloat -1e+04 -5e+02 (Variables|Default|GetIsHitted))) (.x (Math|Vector|GetForwardVector (Transformation|GetActorRotation)))) 0.0 0.0)))

(fn ConstructionScript)