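; BP_Knife is a flying knife actor that awards score to the first-person character when destroyed.
; Each Tick it moves along negative world X at constant speed and tumbles by random roll and yaw increments, with only the movement scaled by delta time.
; BeginPlay caches the player character, and the Destroyed event plays a metal sound and increases that character's Score, whatever caused the destruction.
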(event EventBeginPlay
  (bind _asfirst_person_character (Utilities|Casting|CastToFirstPersonCharacter (Game|GetPlayerCharacter 0)))
  (Variables|Default|SetCharacterREF _asfirst_person_character))

(event EventDestroyed
  (bind _characterref (Variables|Default|GetCharacterREF))
  (Audio|PlaySound2D "/Game/Sounds/C_Metal.C_Metal" 1.0 1.0 0.0 0 0)
  (Variables|/Game/FirstPersonBP/Blueprints/FirstPersonCharacter.FirstPersonCharacter_C|SetScore _characterref (+ (Variables|/Game/FirstPersonBP/Blueprints/FirstPersonCharacter.FirstPersonCharacter_C|GetScore _characterref) 10)))

(event EventTick
  (params (DeltaSeconds :type Float%20%28single-precision%29))
  (bind _returnvalue (Math|Random|RandomFloatinRange 1e+01 2e+01))
  (Transformation|AddActorWorldOffset (Math|Vector|MakeVector (* DeltaSeconds -5e+02) 0.0 0.0))
  (Class|Actor|AddActorWorldRotation (Math|Rotator|MakeRotator _returnvalue 0.0 _returnvalue)))

(fn ConstructionScript)