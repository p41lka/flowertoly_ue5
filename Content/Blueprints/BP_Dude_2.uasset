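; BP_Dude_2 is a child Blueprint for a dude character variant that throws and can be interacted with for points.
; It keeps the parent's BeginPlay and construction logic, adding only its own reactions to two events.
; The ParentShoot event plays the Dude2 throw montage on the skeletal mesh.
; The Interaction event awards a fixed score, then calls Death.
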(event EventBeginPlay
  (|CallParentFunction))

(event Collision|EventActorBeginOverlap
  (params (OtherActor :type Actor%20Object%20Reference))
  (|CallParentFunction OtherActor) ; This node is disabled and will not be called.\nDrag off pins to build functionality.
)

(event EventTick
  (params (DeltaSeconds :type Float%20%28single-precision%29))
  (|CallParentFunction DeltaSeconds) ; This node is disabled and will not be called.\nDrag off pins to build functionality.
)

(event EventParentShoot
  (Animation|Montage|PlayMontage (Variables|Default|GetSkeletalMesh) "/Game/Animations/Dude_2/Dude2_ThrowAnim_Montage.Dude2_ThrowAnim_Montage"))

(event EventInteraction
  (CallFunction|AddScore 100)
  (CallFunction|Death))

(fn ConstructionScript
  (|CallParentFunction))