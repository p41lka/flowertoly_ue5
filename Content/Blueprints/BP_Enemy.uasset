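; BP_Enemy is a base enemy that periodically attacks, spawns a flower on death and can award score to the player.
; A looping timer, with its interval randomized once at BeginPlay, traces forward and calls the empty ParentShoot hook unless another BP_Enemy is hit.
; Death spawns BP_SpawnFlower below the enemy, plays a sound and destroys the actor.
; AddScore increments Score on the cached FirstPersonCharacter.
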(event Custom|CheckThrow
  (bind _returnvalue (Transformation|GetActorLocation))
  (bind _outhit (Collision|LineTraceByChannel _returnvalue (+ _returnvalue (* (Transformation|GetActorForwardVector) (Variables|Default|GetFloat))) "TraceTypeQuery1" false 0 "None"))
  (Utilities|Casting|CastToBP_Enemy (.HitActor (Collision|BreakHitResult _outhit))
    (:CastFailed
      (CallFunction|ParentShoot))))

(event Custom|ParentShoot)

(event Custom|Death
  (bind _returnvalue (Transformation|GetActorLocation))
  (Game|SpawnActorfromClass "/Game/Blueprints/BP_SpawnFlower.BP_SpawnFlower_C" (Math|Transform|MakeTransform (Math|Vector|MakeVector (.x _returnvalue) (.y _returnvalue) (- (.z _returnvalue) 1.5e+02)) "0, 0, 0" "1.000000,1.000000,1.000000") "Undefined" 0 0)
  (Audio|PlaySound2D "/Game/Sounds/C_Death_2.C_Death_2" 1.0 1.0 0.0 0 0)
  (Actor|DestroyActor))

(event Custom|AddScore
  (params (Score :type Integer))
  (bind _characterref (Variables|Default|GetCharacterREF))
  (Variables|/Game/FirstPersonBP/Blueprints/FirstPersonCharacter.FirstPersonCharacter_C|SetScore _characterref (+ (Variables|/Game/FirstPersonBP/Blueprints/FirstPersonCharacter.FirstPersonCharacter_C|GetScore _characterref) Score)))

(event EventBeginPlay
  (bind _asfirst_person_character (Utilities|Casting|CastToFirstPersonCharacter (Game|GetPlayerCharacter 0)))
  (Variables|Default|SetCharacterREF _asfirst_person_character)
  (bind _returnvalue (Utilities|Time|SetTimerbyEvent (delegate Custom|CheckThrow) (Math|Random|RandomFloatinRange 5.0 1e+01) true))
  (Variables|Default|SetThrowTimer _returnvalue))

(fn ConstructionScript)